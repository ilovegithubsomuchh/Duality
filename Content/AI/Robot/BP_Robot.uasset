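; Robot AI Blueprint that follows the player, moves to requested locations and releases a held item.
; FollowPlayer re-runs itself on a short delay while ShouldFollow is set, issuing AIMoveTo toward the player whenever out of range.
; MoveToTarget clears ShouldFollow, ending that loop, and sends the robot to the given location.
; Tick detaches a valid HeldItem and restores its collision whenever ShouldHeld is false.
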(event `self.ReceiveBeginPlay`
  (`self.FollowPlayer`))

(event `self.ReceiveTick`
  (params (DeltaSeconds :type "Float (single-precision)"))
  (bind _helditem (`self.HeldItem`))
  (`/Engine/EditorBlueprintResources/StandardMacros.IsValid` _helditem
    (:`Is Valid`
      (if (not (`self.ShouldHeld`))
        (`self.K2_DetachFromActor` _helditem "KeepWorld" "KeepWorld" "KeepWorld")
        (`self.SetActorEnableCollision` (`self.HeldItem`) true)))))

(event `MoveToTarget`
  (params (TargetLocation :type "Vector Structure"))
  (set `self.ShouldFollow` false)
  (`|AIMoveTo` self TargetLocation null))

(event `FollowPlayer`
  (bind _returnvalue (`GameplayStatics.GetPlayerCharacter` 0))
  (if (`self.ShouldFollow`)
    (if (not (< (`self.GetDistanceTo` _returnvalue) 300.0))
      (`|AIMoveTo` self (0.0 0.0 0.0) _returnvalue 200.0
        (:`then`
          _)))
    (`KismetSystemLibrary.Delay` 0.2)
    (`self.FollowPlayer`)))

(fn `UserConstructionScript`)