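; BP_Camera is a sweeping security camera that sends the player back to the last checkpoint when it spots them.
; While searching, Tick swings Cube1's world yaw back and forth within a fixed arc at constant speed.
; PawnSensing switches the state to Found for pawns tagged Player.
; The next Tick moves the character to the game mode's LastCheckPoint, then resumes searching.
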(event `self.ReceiveTick`
  (params (DeltaSeconds :type "Float (single-precision)"))
  (switch `/Game/_Game/_Core/Element/E_CameraState` (`self.CameraState`)
    (:`NewEnumerator0`
      (`self.RotateCamera`))
    (:`NewEnumerator1`
      (`self.GameOver`))))

(event `RotateCamera`
  (bind _returnvalue (`SceneComponent.K2_GetComponentRotation` (`self.Cube1`)))
  (bind _returnvalue_2 (* (`GameplayStatics.GetWorldDeltaSeconds`) 30.0))
  (bind _yaw (.yaw _returnvalue))
  (bind _yaw_2 (.yaw _returnvalue))
  (set `self.SouldCameraRotateRight` (or (and (< _yaw 30.0) (`self.SouldCameraRotateRight`)) (and (< _yaw -30.0) (not (`self.SouldCameraRotateRight`)))))
  (`SceneComponent.K2_SetWorldRotation` (`self.Cube1`) (`KismetMathLibrary.MakeRotator` (.roll _returnvalue) (.pitch _returnvalue) (`KismetMathLibrary.SelectFloat` (+ _yaw_2 _returnvalue_2) (- _yaw_2 _returnvalue_2) (`self.SouldCameraRotateRight`))) false false))

(event `GameOver`
  (`KismetSystemLibrary.PrintString` "GameOver" true true (struct :`G` 0.66 :`B` 1.0 :`A` 1.0) 0.0)
  (bind _asbp_third_person_game_mode (cast `/Game/_Game/_Core/Player/BP_ThirdPersonGameMode` (`GameplayStatics.GetGameMode`)))
  (bind _asbp_third_person_character (cast `/Game/_Game/_Core/Player/BP_ThirdPersonCharacter` (`GameplayStatics.GetPlayerCharacter` 0)))
  (`SceneComponent.K2_SetWorldLocation` (`Actor.RootComponent` _asbp_third_person_character) (`self.K2_GetActorLocation` (`/Game/_Game/_Core/Player/BP_ThirdPersonGameMode.LastCheckPoint` _asbp_third_person_game_mode)) false false)
  (set `self.CameraState` "NewEnumerator0"))

(event `self.PawnSensing.OnSeePawn`
  (params (Pawn :type "Pawn Object Reference"))
  (if (`self.ActorHasTag` Pawn "Player")
    (set `self.CameraState` "NewEnumerator1")))

(fn `UserConstructionScript`)